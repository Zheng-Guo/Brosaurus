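; Enemy jet fighter that makes a single missile attack run on the player, then climbs away and despawns.
; While Enroute it re-aims its Box at the player's camera every tick; within FireRange it spawns a Missile homing on that camera.
; It then activates UpThuster with higher damping until pitch exceeds 20 degrees, and destroys itself beyond RetreatRange.
; Mesh hits or depleted Durability destroy it with an explosion.
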(event OnComponentHit(StaticMesh)
  (params (HitComponent :type Primitive%20Component%20Object%20Reference) (OtherActor :type Actor%20Object%20Reference) (OtherComp :type Primitive%20Component%20Object%20Reference) (NormalImpulse :type Vector :default "0, 0, 0") (Hit :type Hit%20Result%20Structure%20%28by%20ref%29))
  (Effects|SpawnEmitteratLocation "/Game/StarterContent/Particles/P_Explosion.P_Explosion" (Transformation|GetActorLocation))
  (Actor|DestroyActor))

(event EventBeginPlay
  (CallFunction|Recalibrate))

(event Collision|EventActorBeginOverlap
  (params (OtherActor :type Actor%20Object%20Reference)))

(event EventTick
  (params (DeltaSeconds :type Float%20%28single-precision%29))
  (bind _returnvalue (Game|Player|GetPlayerPawn 0))
  (bind _returnvalue_2 (Transformation|GetActorLocation))
  (bind _returnvalue_3 (Transformation|GetActorLocation _returnvalue))
  (bind _returnvalue_4 (- _returnvalue_3 _returnvalue_2))
  (bind _returnvalue_5 (Math|Vector|VectorLength _returnvalue_4))
  (if (Variables|Default|GetEnroute)
    (if (< (Variables|Default|GetFireRange) _returnvalue_5)
      (CallFunction|Recalibrate)
      (else
        (Variables|Default|SetEnroute false)
        (bind _returnvalue_6 (Game|SpawnActorfromClass "/Game/Blueprints/Missile.Missile_C" (Math|Transform|MakeTransform (- _returnvalue_2 (Math|Vector|MakeVector 0.0 0.0 1e+01)) (Transformation|GetActorRotation) "0.500000,0.500000,0.500000") "Undefined" 0 0))
        (bind _asmy_character (Utilities|Casting|CastToMyCharacter (Game|Player|GetPlayerPawn 0)))
        (Variables|/Script/Engine.ProjectileMovementComponent|SetHomingTargetComponent (Variables|/Game/Blueprints/Missile.Missile_C|GetProjectileMovement _returnvalue_6) (Variables|/Game/Blueprints/MyCharacter.MyCharacter_C|GetCamera _asmy_character))
        (Components|Activation|SetActive (Variables|Default|GetUpThuster) true false)
        (Class|PrimitiveComponent|SetLinearDamping (Variables|Default|GetBox) 0.4)))
    (elif (> (.pitch (Transformation|GetActorRotation)) 2e+01)
      (Components|Activation|SetActive (Variables|Default|GetUpThuster) false false)
      (Class|PrimitiveComponent|SetLinearDamping (Variables|Default|GetBox) 0.1)
      (if (> _returnvalue_5 (Variables|Default|GetRetreatRange))
        (Actor|DestroyActor)))))

(event EventTakeDamage
  (params (Damage :type Float%20%28single-precision%29))
  (Variables|Default|SetDurability (- (Variables|Default|GetDurability) Damage))
  (if (<= (Variables|Default|GetDurability) 0.0)
    (Effects|SpawnEmitteratLocation "/Game/StarterContent/Particles/P_Explosion.P_Explosion" (Transformation|GetActorLocation))
    (Actor|DestroyActor)))

(fn ConstructionScript)

(fn Recalibrate
  (bind _asmy_character (Utilities|Casting|CastToMyCharacter (Game|Player|GetPlayerPawn 0)))
  (Transformation|SetWorldRotation (Variables|Default|GetBox) (Math|Rotator|MakeRotfromX (Math|Vector|GetUnitDirection(Vector) (Transformation|GetActorLocation) (Transformation|GetWorldLocation (Variables|/Game/Blueprints/MyCharacter.MyCharacter_C|GetCamera _asmy_character)))) false false))