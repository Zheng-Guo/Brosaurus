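; Behavior tree task that makes an AI tank chase the player until it has a clear shot.
; Each tick, while the player is within guarding range, a thin capsule trace runs forward, raised by the fire angle.
; If it hits the player within fire range, the tank moves to its own location to halt and succeeds; otherwise it keeps pursuing.
; The task fails once the player is outside guarding range.
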(event EventReceiveTickAI
  (params (OwnerController :type AI%20Controller%20Object%20Reference) (ControlledPawn :type Pawn%20Object%20Reference) (DeltaSeconds :type Float%20%28single-precision%29))
  (bind _returnvalue (Game|Player|GetPlayerPawn 0))
  (bind _returnvalue_2 (Transformation|GetActorLocation ControlledPawn))
  (bind _returnvalue_3 (Transformation|GetActorForwardVector ControlledPawn))
  (bind _firerange (Variables|Default|GetFireRange))
  (bind _returnvalue_4 (Transformation|GetHorizontalDistanceTo ControlledPawn _returnvalue))
  (if (> (Variables|Default|GetGuardingRange) _returnvalue_4)
    (bind _outhit (Class|KismetSystemLibrary|CapsuleTraceSingleNEW (+ _returnvalue_2 (* _returnvalue_3 1.2e+02)) (+ (* _returnvalue_3 _firerange) _returnvalue_2 (Math|Vector|MakeVector 0.0 0.0 (* _firerange (Math|Trig|Tan(Degrees) (Variables|Default|GetFireAngle))))) 3.0 0.0 "TraceTypeQuery2" false 0 "None" true))
    (if (and (== (.HitActor (Collision|BreakHitResult _outhit)) _returnvalue) (<= _returnvalue_4 (Variables|Default|GetFireRange)))
      (AI|AIMoveTo ControlledPawn _returnvalue_2 0 5.0 false
        (:then
          (AI|BehaviorTree|FinishExecute true)))
      (else
        (AI|AIMoveTo ControlledPawn "0, 0, 0" _returnvalue 3e+01 false)))
    (else
      (AI|BehaviorTree|FinishExecute false))))