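; Player character with camera-relative left and right punches, a fireball and a held energy beam, plus standard move and look input.
; Timelines thrust each arm along the camera's forward vector, and overlaps during a punch damage actors implementing the Damageable interface.
; Fireballs and the mouth-attached beam spend a shared Energy pool, which Tick regenerates up to a cap, destroying the beam when energy runs out.
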(event OnComponentBeginOverlap(LeftArm)
  (params (OverlappedComponent :type Primitive%20Component%20Object%20Reference) (OtherActor :type Actor%20Object%20Reference) (OtherComp :type Primitive%20Component%20Object%20Reference) (OtherBodyIndex :type Integer) (bFromSweep :type Boolean) (SweepResult :type Hit%20Result%20Structure%20%28by%20ref%29))
  (if (and (Utilities|DoesObjectImplementInterface OtherActor "/Game/Blueprints/Damageable.Damageable_C") (Variables|Default|GetLeftPunching))
    (Class|Damageable|TakeDamage(Message) OtherActor (Variables|Default|GetPunchDamage))))

(event OnComponentBeginOverlap(RightArm)
  (params (OverlappedComponent :type Primitive%20Component%20Object%20Reference) (OtherActor :type Actor%20Object%20Reference) (OtherComp :type Primitive%20Component%20Object%20Reference) (OtherBodyIndex :type Integer) (bFromSweep :type Boolean) (SweepResult :type Hit%20Result%20Structure%20%28by%20ref%29))
  (if (and (Utilities|DoesObjectImplementInterface OtherActor "/Game/Blueprints/Damageable.Damageable_C") (Variables|Default|GetRightPunching))
    (Class|Damageable|TakeDamage(Message) OtherActor (Variables|Default|GetPunchDamage))))

(event EventBeginPlay
  (bind _camera (Variables|Default|GetCamera))
  (bind _returnvalue (Transformation|GetWorldLocation _camera))
  (Variables|Default|SetLeftArmOffset (- (Transformation|GetWorldLocation (Variables|Default|GetLeftArm)) _returnvalue))
  (Variables|Default|SetRightArmOffset (- (Transformation|GetWorldLocation (Variables|Default|GetRightArm)) _returnvalue))
  (bind _returnvalue_2 (UserInterface|CreateWidget "/Game/Blueprints/MyWidget.MyWidget_C"))
  (UserInterface|Viewport|AddtoViewport _returnvalue_2 0))

(event Collision|EventActorBeginOverlap
  (params (OtherActor :type Actor%20Object%20Reference)))

(event EventTick
  (params (DeltaSeconds :type Float%20%28single-precision%29))
  (bind _beamenergycost (Variables|Default|GetBeamEnergyCost))
  (bind _totalenergy (Variables|Default|GetTotalEnergy))
  (bind _returnvalue (* DeltaSeconds _beamenergycost))
  (if (Variables|Default|GetEnegyBeamActive)
    (if (>= (Variables|Default|GetEnergy) _returnvalue)
      (Variables|Default|SetEnergy (- (Variables|Default|GetEnergy) _returnvalue))
      (if (< (+ (* DeltaSeconds (Variables|Default|GetEnergyRecoverRage)) (Variables|Default|GetEnergy)) _totalenergy) :!label _label
        (Variables|Default|SetEnergy (+ (* DeltaSeconds (Variables|Default|GetEnergyRecoverRage)) (Variables|Default|GetEnergy)))
        (else
          (Variables|Default|SetEnergy _totalenergy)))
      (else
        (Variables|Default|SetEnergy 0.0)
        (Actor|DestroyActor (Variables|Default|GetBeam))
        (Variables|Default|SetEnegyBeamActive false)))
    (else
      (goto _label))))

(event Input|ActionEvents|InputActionEnergyBeam
  (params (Key :type Key%20Structure :default "AnyKey"))
  (bind _mouth (Variables|Default|GetMouth))
  (:Pressed
    (Variables|Default|SetEnegyBeamActive true)
    (bind _returnvalue (Game|SpawnActorfromClass "/Game/Blueprints/EnergyBeam.EnergyBeam_C" (Math|Transform|MakeTransform (Transformation|GetWorldLocation _mouth) (Transformation|GetWorldRotation _mouth) "1,1,1") "Undefined" 0 0))
    (bind _output_get (Variables|Default|SetBeam _returnvalue))
    (Transformation|AttachComponentToComponent _returnvalue (Variables|Default|GetMouth) "None" "SnapToTarget" "SnapToTarget" "KeepRelative" true))
  (:Released
    (if (Utilities|IsValid _output_get)
      (Actor|DestroyActor _returnvalue)
      (Variables|Default|SetEnegyBeamActive false))))

(event Input|ActionEvents|InputActionLeftPunch
  (params (Key :type Key%20Structure :default "AnyKey"))
  (bind _camera (Variables|Default|GetCamera))
  (:Pressed
    (Utilities|FlowControl|DoOnce false :!label _label
      (:Completed
        (Variables|Default|SetLeftPunching true)
        (bind _punch (Timeline|Timeline_0 PlayFromStart)
          (:Update
            (Transformation|SetWorldLocation (Variables|Default|GetLeftArm) (+ (+ (Math|Vector|RotateVector (Variables|Default|GetLeftArmOffset) (Transformation|GetWorldRotation _camera)) (Transformation|GetWorldLocation _camera)) (* (* (Math|Vector|GetForwardVector _camera) _punch) 8e+01)) false false)
            (if (== _punch 1.0)
              (Variables|Default|SetLeftPunching false)))
          (:Finished
            (goto _label Reset)))))))

(event Input|ActionEvents|InputActionRightPunch
  (params (Key :type Key%20Structure :default "AnyKey"))
  (bind _camera (Variables|Default|GetCamera))
  (:Pressed
    (Utilities|FlowControl|DoOnce false :!label _label
      (:Completed
        (Variables|Default|SetRightPunching true)
        (bind _punch (Timeline|Timeline_1 PlayFromStart)
          (:Update
            (Transformation|SetWorldLocation (Variables|Default|GetRightArm) (+ (+ (Math|Vector|RotateVector (Variables|Default|GetRightArmOffset) (Transformation|GetWorldRotation _camera)) (Transformation|GetWorldLocation _camera)) (* (* (Math|Vector|GetForwardVector _camera) _punch) 8e+01)) false false)
            (if (== _punch 1.0)
              (Variables|Default|SetRightPunching false)))
          (:Finished
            (goto _label Reset)))))))

(event Input|ActionEvents|InputActionFire
  (params (Key :type Key%20Structure :default "AnyKey"))
  (:Pressed
    (if (>= (Variables|Default|GetEnergy) (Variables|Default|GetFireballEnergyCost))
      (Variables|Default|SetEnergy (- (Variables|Default|GetEnergy) (Variables|Default|GetFireballEnergyCost)))
      (Game|SpawnActorfromClass "/Game/Blueprints/Fireball.Fireball_C" (Math|Transform|MakeTransform (Transformation|GetWorldLocation (Variables|Default|GetMouth)) (Transformation|GetWorldRotation (Variables|Default|GetCamera)) "0.500000,0.500000,0.500000") "Undefined" 0 0))))

(event Input|AxisEvents|InputAxisMoveForward
  (params (AxisValue :type Float%20%28single-precision%29))
  (Pawn|Input|AddMovementInput (Transformation|GetActorForwardVector) AxisValue true))

(event Input|AxisEvents|InputAxisLookUp
  (params (AxisValue :type Float%20%28single-precision%29))
  (Pawn|Input|AddControllerPitchInput AxisValue)
  (Variables|Default|SetAimingDirection (Math|Vector|RotateVector (Transformation|GetActorForwardVector) (Transformation|GetWorldRotation (Variables|Default|GetCamera)))))

(event Input|AxisEvents|InputAxisLookRight
  (params (AxisValue :type Float%20%28single-precision%29))
  (Pawn|Input|AddControllerYawInput AxisValue)
  (Variables|Default|SetAimingDirection (Math|Vector|RotateVector (Transformation|GetActorForwardVector) (Transformation|GetWorldRotation (Variables|Default|GetCamera)))))

(event Input|AxisEvents|InputAxisMoveRight
  (params (AxisValue :type Float%20%28single-precision%29))
  (Pawn|Input|AddMovementInput (Transformation|GetActorRightVector) AxisValue true))

(fn ConstructionScript)