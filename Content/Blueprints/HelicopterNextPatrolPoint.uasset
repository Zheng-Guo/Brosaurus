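; Behavior Tree task that advances a Chopper to the next point on its patrol route.
; On execute it gets the Chopper from its ChopperController, increments the PatrolPointIndex blackboard value, and wraps to zero past the end of the PatrolPoints array.
; It writes that point to the Destination key, stores the new index, and finishes successfully.
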(event EventReceiveExecute
  (params (OwnerActor :type Actor%20Object%20Reference))
  (bind _patrolpointindex (Variables|Default|GetPatrolPointIndex))
  (bind _returnvalue (Class|BTFunctionLibrary|GetBlackboardValueasInt _patrolpointindex))
  (bind _returnvalue_2 (+ _returnvalue 1))
  (bind _aschopper_controller (Utilities|Casting|CastToChopperController OwnerActor))
  (bind _aschopper (Utilities|Casting|CastToChopper (Pawn|GetControlledPawn _aschopper_controller)))
  (if (>= _returnvalue_2 (Utilities|Array|Length (Variables|/Game/Blueprints/Chopper.Chopper_C|GetPatrolPoints _aschopper)))
    (Variables|Default|SetIndex 0)
    (else
      (Variables|Default|SetIndex _returnvalue_2)))
  (Class|BTFunctionLibrary|SetBlackboardValueasObject (Variables|Default|GetDestination) (Utilities|Array|Get(acopy) (Variables|/Game/Blueprints/Chopper.Chopper_C|GetPatrolPoints _aschopper) (Variables|Default|GetIndex)))
  (Class|BTFunctionLibrary|SetBlackboardValueasInt _patrolpointindex (Variables|Default|GetIndex))
  (AI|BehaviorTree|FinishExecute true))