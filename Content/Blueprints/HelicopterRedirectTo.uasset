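; Behavior tree task that rotates an AI-controlled Chopper to face the Destination actor from the blackboard.
; On execute, if the yaw error exceeds ToleranceAngle, it starts a left or right turn and stops movement.
; Each tick rechecks the error; once within tolerance, it stops turning, snaps yaw onto the target and finishes successfully.
; AngleOfRotation supplies the signed shortest yaw difference, ignoring height.
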(event EventReceiveExecute
  (params (OwnerActor :type Actor%20Object%20Reference))
  (bind _aschopper_controller (Utilities|Casting|CastToChopperController OwnerActor))
  (bind _aschopper (Utilities|Casting|CastToChopper (Pawn|GetControlledPawn _aschopper_controller)))
  (bind _asactor (Utilities|Casting|CastToActor (Class|BTFunctionLibrary|GetBlackboardValueasObject (Variables|Default|GetDestination))))
  (bind _angle (CallFunction|AngleOfRotation _aschopper _asactor))
  (if (> (Math|Float|Absolute(Float) _angle) (Variables|Default|GetToleranceAngle))
    (if (> _angle 0.0)
      (Default|TurnLeft _aschopper)
      (else
        (Default|TurnRight _aschopper)))
    (Default|StopMoving _aschopper)))

(event EventTick
  (params (OwnerActor :type Actor%20Object%20Reference) (DeltaSeconds :type Float%20%28single-precision%29))
  (bind _aschopper_controller (Utilities|Casting|CastToChopperController OwnerActor))
  (bind _aschopper (Utilities|Casting|CastToChopper (Pawn|GetControlledPawn _aschopper_controller)))
  (bind _asactor (Utilities|Casting|CastToActor (Class|BTFunctionLibrary|GetBlackboardValueasObject (Variables|Default|GetDestination))))
  (bind _angle (CallFunction|AngleOfRotation _aschopper _asactor))
  (if (not (> (Math|Float|Absolute(Float) _angle) (Variables|Default|GetToleranceAngle)))
    (Default|StopTurning _aschopper)
    (Transformation|SetActorRotation _aschopper (Math|Rotator|MakeRotator (.roll (Transformation|GetActorRotation _aschopper)) (.pitch (Transformation|GetActorRotation _aschopper)) (- (.yaw (Transformation|GetActorRotation _aschopper)) _angle)))
    (AI|BehaviorTree|FinishExecute true)))

(fn AngleOfRotation
  (params (Actor1 :type Actor%20Object%20Reference) (Actor2 :type Actor%20Object%20Reference))
  (bind _returnvalue (Transformation|GetActorLocation Actor1))
  (bind _returnvalue_2 (Transformation|GetActorLocation Actor2))
  (bind _returnvalue_3 (Transformation|GetActorRotation Actor1))
  (bind _returnvalue_4 (Math|Rotator|FindLookatRotation (Math|Vector|MakeVector (.x _returnvalue) (.y _returnvalue) (.z _returnvalue)) (Math|Vector|MakeVector (.x _returnvalue_2) (.y _returnvalue_2) (.z _returnvalue))))
  (if (< (.yaw _returnvalue_3) 0.0)
    (LocalVariables|SetFromAngle (+ (.yaw _returnvalue_3) 3.6e+02))
    (else
      (LocalVariables|SetFromAngle (.yaw _returnvalue_3))))
  (if (< (.yaw _returnvalue_4) 0.0)
    (LocalVariables|SetToAngle (+ (.yaw _returnvalue_4) 3.6e+02))
    (else
      (LocalVariables|SetToAngle (.yaw _returnvalue_4))))
  (if (> (- (LocalVariables|GetFromAngle) (LocalVariables|GetToAngle)) 1.8e+02)
    (LocalVariables|SetResult (- (- (LocalVariables|GetFromAngle) (LocalVariables|GetToAngle)) 3.6e+02))
    (elif (< (- (LocalVariables|GetFromAngle) (LocalVariables|GetToAngle)) -1.8e+02)
      (LocalVariables|SetResult (+ (- (LocalVariables|GetFromAngle) (LocalVariables|GetToAngle)) 3.6e+02))
      (else
        (LocalVariables|SetResult (- (LocalVariables|GetFromAngle) (LocalVariables|GetToAngle))))))
  (return (LocalVariables|GetResult)))