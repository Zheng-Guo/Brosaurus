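; CivilianCar is a civilian vehicle actor that is given a destination through an AI blackboard and can be destroyed by damage.
; On BeginPlay it writes its Destination vector into the blackboard's "Destination" key.
; Incoming damage reduces Durability, and at zero or below the car spawns an explosion emitter at its location and destroys itself.
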(event EventBeginPlay
  (AI|Components|Blackboard|SetValueasVector (AI|GetBlackboard self) (Utilities|Name|MakeLiteralName "Destination") (Variables|Default|GetDestination)))

(event Collision|EventActorBeginOverlap
  (params (OtherActor :type Actor%20Object%20Reference)))

(event EventTakeDamage
  (params (Damage :type Float%20%28single-precision%29))
  (Variables|Default|SetDurability (- (Variables|Default|GetDurability) Damage))
  (if (<= (Variables|Default|GetDurability) 0.0)
    (Effects|SpawnEmitteratLocation "/Game/StarterContent/Particles/P_Explosion.P_Explosion" (Transformation|GetActorLocation))
    (Actor|DestroyActor)))

(event EventTick
  (params (DeltaSeconds :type Float%20%28single-precision%29)))

(fn ConstructionScript)