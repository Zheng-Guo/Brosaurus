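; Behavior tree task that flies an AI-controlled Chopper until it is within an acceptable horizontal radius of the Destination blackboard actor.
; On execute it starts the Chopper moving forward unless already in range; the task itself does no steering.
; Tick rechecks the distance, then stops the Chopper and finishes successfully once inside the radius.
; A failed cast exits silently, and the task has no failure result.
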(event EventReceiveExecute
  (params (OwnerActor :type Actor%20Object%20Reference))
  (bind _aschopper_controller (Utilities|Casting|CastToChopperController OwnerActor))
  (bind _aschopper (Utilities|Casting|CastToChopper (Pawn|GetControlledPawn _aschopper_controller)))
  (bind _asactor (Utilities|Casting|CastToActor (Class|BTFunctionLibrary|GetBlackboardValueasObject (Variables|Default|GetDestination))))
  (if (not (< (Transformation|GetHorizontalDistanceTo _asactor _aschopper) (Variables|Default|GetAcceptableRadius)))
    (Default|MoveForward _aschopper)))

(event EventTick
  (params (OwnerActor :type Actor%20Object%20Reference) (DeltaSeconds :type Float%20%28single-precision%29))
  (bind _aschopper_controller (Utilities|Casting|CastToChopperController OwnerActor))
  (bind _aschopper (Utilities|Casting|CastToChopper (Pawn|GetControlledPawn _aschopper_controller)))
  (bind _asactor (Utilities|Casting|CastToActor (Class|BTFunctionLibrary|GetBlackboardValueasObject (Variables|Default|GetDestination))))
  (if (< (Transformation|GetHorizontalDistanceTo _asactor _aschopper) (Variables|Default|GetAcceptableRadius))
    (Default|StopMoving _aschopper)
    (AI|BehaviorTree|FinishExecute true)))