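; EnergyBeam is a continuous breath-beam attack that fires forward from a Mouth component using the P_AtomaticBreath particle effect.
; BeginPlay attaches the emitter to Mouth and sets its initial end point.
; Each Tick, a capsule multi-trace clips the beam at a blocking hit, or leaves it at full range.
; Non-blocking hit actors implementing the Damageable interface receive frame-time-scaled damage, while blocking hits take none.
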(event EventBeginPlay
  (bind _mouth (Variables|Default|GetMouth))
  (bind _firerange (Variables|Default|GetFireRange))
  (bind _returnvalue (Transformation|GetWorldLocation _mouth))
  (bind _returnvalue_2 (Math|Vector|GetForwardVector _mouth))
  (bind _returnvalue_3 (* _returnvalue_2 _firerange))
  (bind _returnvalue_4 (+ _returnvalue _returnvalue_3))
  (bind _returnvalue_5 (Effects|SpawnEmitterAttached "/Game/ExampleContent/Effects/ParticleSystems/P_AtomaticBreath.P_AtomaticBreath" _mouth "None"))
  (bind _output_get (Variables|Default|SetBeam _returnvalue_5))
  (Variables|Default|SetDestination _returnvalue_4)
  (bind _outhits (Class|KismetSystemLibrary|CapsuleTraceMultiNEW _returnvalue _returnvalue_4 (Variables|Default|GetDamageRange) 0.0 "TraceTypeQuery3" false 0 "None" true))
  (for _array_element _outhits
    (if (.bBlockingHit (Collision|BreakHitResult _array_element))
      (Variables|Default|SetDestination (.ImpactPoint (Collision|BreakHitResult _array_element)))))
  (Class|ParticleSystemComponent|SetBeamEndPoint _output_get 0 (Variables|Default|GetDestination)))

(event EventTick
  (params (DeltaSeconds :type Float%20%28single-precision%29))
  (bind _mouth (Variables|Default|GetMouth))
  (bind _firerange (Variables|Default|GetFireRange))
  (bind _returnvalue (Transformation|GetWorldLocation _mouth))
  (bind _returnvalue_2 (Math|Vector|GetForwardVector _mouth))
  (bind _returnvalue_3 (* _returnvalue_2 _firerange))
  (bind _returnvalue_4 (+ _returnvalue _returnvalue_3))
  (Variables|Default|SetDestination _returnvalue_4)
  (bind _outhits (Class|KismetSystemLibrary|CapsuleTraceMultiNEW _returnvalue _returnvalue_4 (Variables|Default|GetDamageRange) 0.0 "TraceTypeQuery3" false 0 "None" true))
  (for _array_element _outhits
    (if (.bBlockingHit (Collision|BreakHitResult _array_element))
      (Variables|Default|SetDestination (.ImpactPoint (Collision|BreakHitResult _array_element)))
      (elif (Utilities|DoesObjectImplementInterface (.HitActor (Collision|BreakHitResult _array_element)) "/Game/Blueprints/Damageable.Damageable_C")
        (Class|Damageable|TakeDamage(Message) (.HitActor (Collision|BreakHitResult _array_element)) (* DeltaSeconds (Variables|Default|GetDamage))))))
  (Class|ParticleSystemComponent|SetBeamEndPoint (Variables|Default|GetBeam) 0 (Variables|Default|GetDestination)))

(fn ConstructionScript)