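; Behavior tree task that makes an AI-controlled Chopper chase the blackboard Enemy until it is within firing range.
; On execute it starts moving forward if the enemy is out of FireRange.
; Each tick it turns to face the enemy on the horizontal plane and keeps moving forward.
; It stops and succeeds inside FireRange, and fails once the horizontal distance is no longer within GuardingRadius.
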(event EventReceiveExecute
  (params (OwnerActor :type Actor%20Object%20Reference))
  (bind _aschopper_controller (Utilities|Casting|CastToChopperController OwnerActor))
  (bind _aschopper (Utilities|Casting|CastToChopper (Pawn|GetControlledPawn _aschopper_controller)))
  (bind _asactor (Utilities|Casting|CastToActor (Class|BTFunctionLibrary|GetBlackboardValueasObject (Variables|Default|GetEnemy))))
  (if (not (< (Transformation|GetHorizontalDistanceTo _asactor _aschopper) (Variables|Default|GetFireRange)))
    (Default|MoveForward _aschopper)))

(event EventTick
  (params (OwnerActor :type Actor%20Object%20Reference) (DeltaSeconds :type Float%20%28single-precision%29))
  (bind _aschopper_controller (Utilities|Casting|CastToChopperController OwnerActor))
  (bind _aschopper (Utilities|Casting|CastToChopper (Pawn|GetControlledPawn _aschopper_controller)))
  (bind _asactor (Utilities|Casting|CastToActor (Class|BTFunctionLibrary|GetBlackboardValueasObject (Variables|Default|GetEnemy))))
  (if (< (Transformation|GetHorizontalDistanceTo _asactor _aschopper) (Variables|Default|GetGuardingRadius))
    (if (< (Transformation|GetHorizontalDistanceTo _asactor _aschopper) (Variables|Default|GetFireRange))
      (Default|StopMoving _aschopper)
      (AI|BehaviorTree|FinishExecute true)
      (else
        (Transformation|SetActorRotation _aschopper (Math|Rotator|MakeRotfromX (Math|Vector|GetUnitDirection(Vector) (Math|Vector|MakeVector (.x (Transformation|GetActorLocation _aschopper)) (.y (Transformation|GetActorLocation _aschopper)) (.z (Transformation|GetActorLocation _aschopper))) (Math|Vector|MakeVector (.x (Transformation|GetActorLocation _asactor)) (.y (Transformation|GetActorLocation _asactor)) (.z (Transformation|GetActorLocation _aschopper))))))
        (Default|MoveForward _aschopper)))
    (else
      (AI|BehaviorTree|FinishExecute false))))