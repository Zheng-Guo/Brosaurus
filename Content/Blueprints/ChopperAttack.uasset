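; ChopperAttack is a behavior tree task that has an AI-controlled Chopper attack its enemy when within range.
; On tick, it gets the Chopper from its ChopperController and compares horizontal distance to the blackboard Enemy against FireRange.
; In range, it calls Attack on that enemy and finishes successfully; otherwise it finishes as failed.
; Failed controller or pawn casts stop the tick without finishing the task.
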(event EventReceiveExecute
  (params (OwnerActor :type Actor%20Object%20Reference)))

(event EventTick
  (params (OwnerActor :type Actor%20Object%20Reference) (DeltaSeconds :type Float%20%28single-precision%29))
  (bind _enemy (Variables|Default|GetEnemy))
  (bind _returnvalue (AI|BehaviorTree|GetBlackboardValueasActor _enemy))
  (bind _aschopper_controller (Utilities|Casting|CastToChopperController OwnerActor))
  (bind _aschopper (Utilities|Casting|CastToChopper (Pawn|GetControlledPawn _aschopper_controller)))
  (if (< (Transformation|GetHorizontalDistanceTo _aschopper _returnvalue) (Variables|Default|GetFireRange))
    (Default|Attack _aschopper _returnvalue)
    (AI|BehaviorTree|FinishExecute true)
    (else
      (AI|BehaviorTree|FinishExecute false))))