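; Building is a destructible structure actor that takes damage, catches fire when weakened, and explodes when destroyed.
; The construction script applies the configurable Mesh to its static mesh component.
; TakeDamage reduces Durability, switches the particle component to a fire effect below BurningThreshold, and at zero spawns an explosion emitter and destroys the actor.
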(event EventBeginPlay)

(event Collision|EventActorBeginOverlap
  (params (OtherActor :type Actor%20Object%20Reference)))

(event EventTick
  (params (DeltaSeconds :type Float%20%28single-precision%29)))

(event EventTakeDamage
  (params (Damage :type Float%20%28single-precision%29))
  (Variables|Default|SetDurability (- (Variables|Default|GetDurability) Damage))
  (if (<= (Variables|Default|GetDurability) 0.0)
    (Effects|SpawnEmitteratLocation "/Game/StarterContent/Particles/P_Explosion.P_Explosion" (Transformation|GetActorLocation))
    (Actor|DestroyActor)
    (elif (< (Variables|Default|GetDurability) (Variables|Default|GetBurningThreshold))
      (Effects|Components|ParticleSystem|SetTemplate (Variables|Default|GetParticleSystem) "/Game/StarterContent/Particles/P_Fire.P_Fire"))))

(fn ConstructionScript
  (Components|StaticMesh|SetStaticMesh (Variables|Default|GetStaticMesh) (Variables|Default|GetMesh)))