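; Behavior tree task that makes an AI-controlled Tank fire at the first player's pawn when it is within range.
; On AI tick it compares the horizontal distance to FireRange and fails if the player is farther away.
; In range, it adds delta time to TimeBetweenShots, calls Attack and resets the timer once FireInterval is reached, and finishes successfully whether or not it fired.
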(event EventReceiveTickAI
  (params (OwnerController :type AI%20Controller%20Object%20Reference) (ControlledPawn :type Pawn%20Object%20Reference) (DeltaSeconds :type Float%20%28single-precision%29))
  (bind _astank (Utilities|Casting|CastToTank ControlledPawn))
  (if (<= (Transformation|GetHorizontalDistanceTo _astank (Game|Player|GetPlayerPawn 0)) (Variables|Default|GetFireRange))
    (if (>= (+ DeltaSeconds (Variables|Default|GetTimeBetweenShots)) (Variables|Default|GetFireInterval))
      (Variables|Default|SetTimeBetweenShots 0.0)
      (Default|Attack _astank)
      (else
        (Variables|Default|SetTimeBetweenShots (+ DeltaSeconds (Variables|Default|GetTimeBetweenShots)))))
    (AI|BehaviorTree|FinishExecute true)
    (else
      (AI|BehaviorTree|FinishExecute false))))