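; AI controller for a Tank pawn that starts its patrol behavior when it takes possession.
; UpdatePatrolPoints sets up TankBlackboard, seeds NextDestination with the tank's first patrol point and PatrolPointIndex with zero, then runs TankBehaviorTree.
; Advancing along the route is not handled here; the controller only sets the starting state.
; The EventGraph also holds an unconnected duplicate of that setup, which never runs.
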(event EventBeginPlay)

(event EventTick
  (params (DeltaSeconds :type Float%20%28single-precision%29)))

(event EventOnPossess
  (params (PossessedPawn :type Pawn%20Object%20Reference))
  (CallFunction|UpdatePatrolPoints))

(fn ConstructionScript)

(fn UpdatePatrolPoints
  (bind _blackboardcomponent (Class|AIController|UseBlackboard "/Game/Blueprints/TankBlackboard.TankBlackboard"))
  (bind _astank (Utilities|Casting|CastToTank (Pawn|GetControlledPawn)))
  (AI|Components|Blackboard|SetValueasObject _blackboardcomponent (Utilities|Name|MakeLiteralName "NextDestination") (Utilities|Array|Get(acopy) (Variables|/Game/Blueprints/Tank.Tank_C|GetPatrolPoints _astank)))
  (Class|BlackboardComponent|SetValueasInt _blackboardcomponent (Utilities|Name|MakeLiteralName "PatrolPointIndex"))
  (AI|RunBehaviorTree "/Game/Blueprints/TankBehaviorTree.TankBehaviorTree"))