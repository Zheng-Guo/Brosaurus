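; An AI controller that drives a Chopper pawn through a behavior tree.
; On BeginPlay it activates the chopper blackboard and seeds it with the pawn's first patrol point as the next destination, a zero patrol index, and the player pawn as the enemy.
; It then runs the chopper behavior tree, stopping early if the controlled pawn is not a Chopper.
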(event EventBeginPlay
  (bind _self self)
  (bind _returnvalue (AI|GetBlackboard _self))
  (Class|AIController|UseBlackboard "/Game/Blueprints/ChopperBlackboard.ChopperBlackboard")
  (bind _aschopper (Utilities|Casting|CastToChopper (Pawn|GetControlledPawn)))
  (AI|Components|Blackboard|SetValueasObject _returnvalue (Utilities|Name|MakeLiteralName "NextDestination") (Utilities|Array|Get(acopy) (Variables|/Game/Blueprints/Chopper.Chopper_C|GetPatrolPoints _aschopper)))
  (Class|BlackboardComponent|SetValueasInt _returnvalue (Utilities|Name|MakeLiteralName "PatrolPointIndex"))
  (AI|Components|Blackboard|SetValueasObject _returnvalue (Utilities|Name|MakeLiteralName "Enemy") (Game|Player|GetPlayerPawn 0))
  (AI|RunBehaviorTree "/Game/Blueprints/ChopperBehaviourTree.ChopperBehaviourTree"))

(fn ConstructionScript)