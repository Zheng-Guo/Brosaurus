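; AtomicBreath actor that fires a beam particle from a Mouth component to a Target and pushes destructible objects in its path.
; The construction script uses FireRange and DamageSection to size and offset the hit Box and place the Target.
; BeginPlay attaches the beam emitter to Mouth, and Tick updates its end point to the Target.
; Destructible components entering the Box receive an impulse along the Mouth-to-Target vector.
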(event OnComponentBeginOverlap(Box)
  (params (OverlappedComponent :type Primitive%20Component%20Object%20Reference) (OtherActor :type Actor%20Object%20Reference) (OtherComp :type Primitive%20Component%20Object%20Reference) (OtherBodyIndex :type Integer) (bFromSweep :type Boolean) (SweepResult :type Hit%20Result%20Structure%20%28by%20ref%29))
  (bind _asdestructible_component (Utilities|Casting|CastToDestructibleComponent OtherComp))
  (Physics|AddImpulse _asdestructible_component (- (Transformation|GetWorldLocation (Variables|Components|GetTarget)) (Transformation|GetWorldLocation (Variables|Default|GetMouth))) "None" false))

(event EventBeginPlay
  (bind _returnvalue (Effects|SpawnEmitterAttached "/Game/ExampleContent/Effects/ParticleSystems/P_AtomaticBreath.P_AtomaticBreath" (Variables|Default|GetMouth) "None"))
  (Variables|Default|SetBeam _returnvalue))

(event Collision|EventActorBeginOverlap
  (params (OtherActor :type Actor%20Object%20Reference)))

(event EventTick
  (params (DeltaSeconds :type Float%20%28single-precision%29))
  (CallFunction|SetDimension))

(fn ConstructionScript
  (bind _damagesection (Variables|Default|GetDamageSection))
  (Transformation|AddLocalOffset (Variables|Default|GetBox) (Math|Vector|MakeVector (Variables|Default|GetFireRange) 0.0 0.0) false false)
  (Components|Box|SetBoxExtent (Variables|Default|GetBox) (Math|Vector|MakeVector (Variables|Default|GetFireRange) _damagesection _damagesection) true)
  (Transformation|AddLocalOffset (Variables|Components|GetTarget) (Math|Vector|MakeVector (Variables|Default|GetFireRange) 0.0 0.0) false false))

(fn SetDimension
  (Class|ParticleSystemComponent|SetBeamTargetPoint (Variables|Default|GetBeam) 0 (Transformation|GetWorldLocation (Variables|Components|GetTarget))))