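; Behavior tree task that advances an AI-controlled Tank to the next point on its patrol route.
; It increments the patrol index stored in the blackboard, wrapping to zero past the end of the Tank's PatrolPoints array.
; It writes that point to the Destination key, saves the new index and finishes with success.
; A pawn that is not a Tank stops execution without finishing the task.
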(event EventReceiveExecuteAI
  (params (OwnerController :type AI%20Controller%20Object%20Reference) (ControlledPawn :type Pawn%20Object%20Reference))
  (bind _patropointindex (Variables|Default|GetPatroPointIndex))
  (bind _returnvalue (Class|BTFunctionLibrary|GetBlackboardValueasInt _patropointindex))
  (bind _returnvalue_2 (+ _returnvalue 1))
  (bind _astank (Utilities|Casting|CastToTank ControlledPawn))
  (if (>= _returnvalue_2 (Utilities|Array|Length (Variables|/Game/Blueprints/Tank.Tank_C|GetPatrolPoints _astank)))
    (Variables|Default|SetIndex 0)
    (else
      (Variables|Default|SetIndex _returnvalue_2)))
  (Class|BTFunctionLibrary|SetBlackboardValueasObject (Variables|Default|GetDestination) (Utilities|Array|Get(acopy) (Variables|/Game/Blueprints/Tank.Tank_C|GetPatrolPoints _astank) (Variables|Default|GetIndex)))
  (Class|BTFunctionLibrary|SetBlackboardValueasInt _patropointindex (Variables|Default|GetIndex))
  (AI|BehaviorTree|FinishExecute true))