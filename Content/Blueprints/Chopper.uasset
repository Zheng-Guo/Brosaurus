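; Chopper is a destructible helicopter that exposes movement, turning and attack functions, with no input or AI logic of its own.
; Movement and turning set linear and angular velocity directly on the physics Box, leaving older AddActorWorldRotation turn nodes unused.
; Attack spawns a HelicopterBullet_BP just ahead of and below the body, aimed at the given Enemy.
; Damage reduces Durability until the chopper spawns an explosion and destroys itself.
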(event EventBeginPlay)

(event Collision|EventActorBeginOverlap
  (params (OtherActor :type Actor%20Object%20Reference)))

(event EventTick
  (params (DeltaSeconds :type Float%20%28single-precision%29)))

(event EventTakeDamage
  (params (Damage :type Float%20%28single-precision%29))
  (Variables|Default|SetDurability (- (Variables|Default|GetDurability) Damage))
  (if (<= (Variables|Default|GetDurability) 0.0)
    (Effects|SpawnEmitteratLocation "/Game/StarterContent/Particles/P_Explosion.P_Explosion" (Transformation|GetActorLocation))
    (Actor|DestroyActor)))

(fn ConstructionScript)

(fn MoveForward
  (Physics|SetPhysicsLinearVelocity (Variables|Default|GetBox) (* (Transformation|GetActorForwardVector) (Variables|Default|GetSpeed)) false "None"))

(fn MoveBackward
  (Physics|SetPhysicsLinearVelocity (Variables|Default|GetBox) (* (Transformation|GetActorForwardVector) (* (Variables|Default|GetSpeed) -1.0)) false "None"))

(fn StopMoving
  (Physics|SetPhysicsLinearVelocity (Variables|Default|GetBox) "0, 0, 0" false "None"))

(fn MoveUp
  (Physics|SetPhysicsLinearVelocity (Variables|Default|GetBox) (* (Transformation|GetActorUpVector) (Variables|Default|GetSpeed)) false "None"))

(fn MoveDown
  (Physics|SetPhysicsLinearVelocity (Variables|Default|GetBox) (* (Transformation|GetActorUpVector) (* (Variables|Default|GetSpeed) -1.0)) false "None"))

(fn MoveLeft
  (Physics|SetPhysicsLinearVelocity (Variables|Default|GetBox) (* (Transformation|GetActorRightVector) (* (Variables|Default|GetSpeed) -1.0)) false "None"))

(fn MoveRight
  (Physics|SetPhysicsLinearVelocity (Variables|Default|GetBox) (* (Transformation|GetActorRightVector) (Variables|Default|GetSpeed)) false "None"))

(fn TurnLeft
  (Class|PrimitiveComponent|SetPhysicsAngularVelocity (Variables|Default|GetBox) (Math|Vector|MakeVector 0.0 0.0 (* (Variables|Default|GetRotatingSpeed) -1.0)) false "None"))

(fn TurnRight
  (Class|PrimitiveComponent|SetPhysicsAngularVelocity (Variables|Default|GetBox) (Math|Vector|MakeVector 0.0 0.0 (Variables|Default|GetRotatingSpeed)) false "None"))

(fn StopTurning
  (Class|PrimitiveComponent|SetPhysicsAngularVelocity (Variables|Default|GetBox) "0, 0, 0" false "None"))

(fn Attack
  (params (Enemy :type Actor%20Object%20Reference))
  (bind _returnvalue (Transformation|GetActorForwardVector))
  (bind _returnvalue_2 (Transformation|GetActorTransform))
  (bind _returnvalue_3 (Transformation|GetActorUpVector))
  (bind _returnvalue_4 (* _returnvalue 5e+01))
  (bind _returnvalue_5 (* _returnvalue_3 -3e+01))
  (bind _returnvalue_6 (+ _returnvalue_4 (.location _returnvalue_2) _returnvalue_5))
  (Game|SpawnActorfromClass "/Game/Blueprints/HelicopterBullet_BP.HelicopterBullet_BP_C" (Math|Transform|MakeTransform _returnvalue_6 (Math|Rotator|MakeRotfromXY (Math|Vector|GetUnitDirection(Vector) _returnvalue_6 (Transformation|GetActorLocation Enemy)) (Transformation|GetActorRightVector)) "0.100000,0.100000,0.100000") "Undefined" 0 0))